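; BP_Bed is an interactable bed actor that starts a screen fade when used.
; EnableInfo and DisableInfo show and hide its InformationWidget component, whose widget is exposed through GetInformationWidget.
; Use requires a PC_StartMain controller, on which it calls StartFade and disables input, then fades out the W_ActorInformation widget, logging when the controller cast fails.
; WhenScreenStartBlack is an empty stub.
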(event EventBeginPlay)

(event EventEnableInfo
  (Rendering|SetVisibility (Variables|Default|GetInformationWidget) true false))

(event EventDisableInfo
  (Rendering|SetVisibility (Variables|Default|GetInformationWidget) false false))

(event EventUse
  (params (PlayerController :type Player%20Controller%20Object%20Reference))
  (bind _aspc_start_main (Utilities|Casting|CastToPC_StartMain PlayerController)
    (:then
      (Default|StartFade _aspc_start_main)
      (Input|DisableInput PlayerController PlayerController)
      (bind _asw_actor_information (Utilities|Casting|CastToW_ActorInformation (UserInterface|GetWidget (Variables|Default|GetInformationWidget))))
      (Default|FadeOutWidget _asw_actor_information))
    (:CastFailed
      (CallFunction|LogInfo "BP_Bed" "Player Controller Not PC_StartMain"))))

(event Collision|EventActorBeginOverlap
  (params (OtherActor :type Actor%20Object%20Reference)))

(fn ConstructionScript)

(fn GetInformationWidget
  (return (UserInterface|GetWidget (Variables|Default|GetInformationWidget))))

(fn WhenScreenStartBlack)