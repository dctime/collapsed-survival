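; BP_CircuitBoard is an actor that builds a circuit board with input and output terminals when play begins.
; It scales the Board component uniformly by BoardSizeOdd, then passes that size with InputAmount and OutputAmount to CalculateInputLocations and CalculateOutputLocations.
; It spawns a BP_InputTerminal or BP_OutputTerminal at each returned location.
; The construction script, Tick and overlap events are empty.
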(event EventBeginPlay
  (bind _boardsizeodd (Variables|Default|GetBoardSizeOdd))
  (bind _returnvalue (Math|Conversions|ToFloat(Integer) _boardsizeodd))
  (Transformation|SetWorldScale3D (Variables|Default|GetBoard) (Math|Vector|MakeVector _returnvalue _returnvalue _returnvalue))
  (bind _returnvalue_2 (Class|CPPCircuitBoard|CalculateInputLocations (Variables|Default|GetBoardSizeOdd) (Variables|Default|GetInputAmount)))
  (for _array_element _returnvalue_2
    (Game|SpawnActorfromClass "/Game/Actors/BP_InputTerminal.BP_InputTerminal_C" (Math|Transform|MakeTransform _array_element "0, 0, 0" "1.000000,1.000000,1.000000") "Undefined" "MultiplyWithRoot" 0 0))
  (bind _returnvalue_3 (Class|CPPCircuitBoard|CalculateOutputLocations (Variables|Default|GetBoardSizeOdd) (Variables|Default|GetOutputAmount)))
  (for _array_element_2 _returnvalue_3
    (Game|SpawnActorfromClass "/Game/Actors/BP_OutputTerminal.BP_OutputTerminal_C" (Math|Transform|MakeTransform _array_element_2 "0, 0, 0" "1.000000,1.000000,1.000000") "Undefined" "MultiplyWithRoot" 0 0)))

(event Collision|EventActorBeginOverlap
  (params (OtherActor :type Actor%20Object%20Reference)))

(event EventTick
  (params (DeltaSeconds :type Float%20%28single-precision%29)))

(fn ConstructionScript)