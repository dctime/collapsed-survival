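; Main character Blueprint that detects and tracks actors in front of the player, with an outline color passed to the detection.
; BeginPlay creates a cancel-collision sphere slightly larger than the use range.
; Each Tick feeds that sphere and the head and feet arrows into DetectForward, along with the detected and closest actor variables.
; A helper searches all beds for one within a given capsule distance, printing each checked distance.
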(event EventBeginPlay
  (bind _returnvalue (AddComponent|AddSphereComponent false))
  (Variables|Default|SetCancelCollision _returnvalue)
  (Components|Sphere|SetSphereRadius _returnvalue (+ (Variables|Default|GetUseRange) 1e+01) true))

(event Collision|EventActorBeginOverlap
  (params (OtherActor :type Actor%20Object%20Reference)))

(event EventTick
  (params (DeltaSeconds :type Float%20%28single-precision%29))
  (Class|CPPMainCharacter|DetectForward (Variables|Default|GetDetectedActors) (Variables|Default|GetClosestDetectedActor) 5 (Variables|Default|GetHeadDetectArrow) (Variables|Default|GetFeetDetectArrow) (Variables|Default|GetCancelCollision) 400 "(R=0.000000,G=0.087691,B=1.000000,A=1.000000)"))

(fn ConstructionScript)

(fn CheckBedNear
  (params (BedDistance :type Float%20%28double-precision%29))
  (bind _outactors (Actor|GetAllActorsOfClass "/Game/Actors/BP_Bed.BP_Bed_C"))
  (for _array_element _outactors
    (Development|PrintString (Utilities|String|ToString(Float) (Math|Vector|VectorLength (- (Transformation|GetWorldLocation (Variables|Default|GetCapsuleComponent)) (Transformation|GetWorldLocation (Variables|/Game/Actors/BP_Bed.BP_Bed_C|GetDefaultSceneRoot _array_element))))))
    (if (< (Math|Vector|VectorLength (- (Transformation|GetWorldLocation (Variables|Default|GetCapsuleComponent)) (Transformation|GetWorldLocation (Variables|/Game/Actors/BP_Bed.BP_Bed_C|GetDefaultSceneRoot _array_element)))) BedDistance)
      (return (< (Math|Vector|VectorLength (- (Transformation|GetWorldLocation (Variables|Default|GetCapsuleComponent)) (Transformation|GetWorldLocation (Variables|/Game/Actors/BP_Bed.BP_Bed_C|GetDefaultSceneRoot _array_element)))) BedDistance) _array_element)))
  (return false 0))