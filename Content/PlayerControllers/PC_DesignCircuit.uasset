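; Player controller for circuit design that previews, rotates and places components on a circuit board.
; BeginPlay shows the cursor and adds the not-selected-mode Enhanced Input context.
; Tick previews a hardcoded BP_Denser on BP_CircuitBoard and puts it in preview mode through BPI_CircuitDesign_CanPlace.
; Place input switches the previewed actor to functioning mode and releases it, while rotate input turns the preview a quarter and logs it.
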(event Input|EnhancedActionEvents|EnhancedInputActionIA_PlaceCircuitComponent
  (params (ActionValue :type Boolean) (ElapsedSeconds :type Float%20%28double-precision%29) (TriggeredSeconds :type Float%20%28double-precision%29) (InputAction :type Input%20Action%20Object%20Reference :default "/Game/InputActions/IA_PlaceCircuitComponent.IA_PlaceCircuitComponent"))
  (:Started
    (Class|BPICircuitDesignCanPlace|ActivateFunctioningMode(Message) (Variables|Default|GetPreviewedActor))
    (Variables|Default|SetPreviewedActor 0)))

(event Input|EnhancedActionEvents|EnhancedInputActionIA_RotatePreview
  (params (ActionValue :type Boolean) (ElapsedSeconds :type Float%20%28double-precision%29) (TriggeredSeconds :type Float%20%28double-precision%29) (InputAction :type Input%20Action%20Object%20Reference :default "/Game/InputActions/IA_RotatePreview.IA_RotatePreview"))
  (:Started
    (Class|CPPPCDesignCircuit|RotatePreviewQuarter)
    (CallFunction|LogInfo "PC_DesignCircuit" "Rotate!")))

(event EventBeginPlay
  (Utilities|FlowControl|Sequence
    (:then_0
      (Variables|Default|SetbShowMouseCursor true))
    (:then_1
      (Input|AddMappingContext (PlayerController|LocalPlayerSubsystems|GetEnhancedInputLocalPlayerSubsystem self) "/Game/InputMappingContext/IMC_DesignCircuit_NotSelectedMode.IMC_DesignCircuit_NotSelectedMode" 0 "(bIgnoreAllPressedKeysUntilRelease=True,bForceImmediately=False,bNotifyUserSettings=False)"))))

(event EventTick
  (params (DeltaSeconds :type Float%20%28single-precision%29))
  (Utilities|FlowControl|Sequence
    (:then_0
      (Class|CPPPCDesignCircuit|PreviewComponentontheBoard "/Game/Actors/BP_Denser.BP_Denser_C" "/Game/Actors/BP_CircuitBoard.BP_CircuitBoard_C"))
    (:then_1
      (bind _asbpi_circuit_design_can_place (Utilities|Casting|CastToBPI_CircuitDesign_CanPlace (Variables|Default|GetPreviewedActor)))
      (Default|ActivatePreviewMode _asbpi_circuit_design_can_place))))

(fn ConstructionScript)