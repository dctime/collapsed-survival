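; Player controller for the Lumina circuit design view, showing the mouse cursor and mapping Enhanced Input to pan, zoom and component placement.
; Move inputs call the inherited Move function at a speed proportional to zoom size.
; Zoom input scales that size multiplicatively within clamped limits and applies it as the controlled character's camera screen size.
; Placement calls PlaceComponent with a fixed value, alongside leftover debug prints.
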(event Input|EnhancedActionEvents|EnhancedInputActionIA_Zoom
  (params (ActionValue :type Float%20%28double-precision%29) (ElapsedSeconds :type Float%20%28double-precision%29) (TriggeredSeconds :type Float%20%28double-precision%29) (InputAction :type Input%20Action%20Object%20Reference :default "/Game/InputActions/IA_Zoom.IA_Zoom"))
  (bind _returnvalue (* ActionValue 2.0))
  (if (> ActionValue 0.0)
    (Variables|Default|SetZoomSize (Math|Float|Clamp(Float) (/ (Variables|Default|GetZoomSize) _returnvalue) 8.0 1024.0))
    (else
      (Variables|Default|SetZoomSize (Math|Float|Clamp(Float) (* (Variables|Default|GetZoomSize) (* _returnvalue -1.0)) 8.0 1024.0))
      (Development|PrintString "Zoom Out")))
  (CallFunction|BPZoom (Variables|Default|GetZoomSize))
  (Development|PrintString (Utilities|String|ToString(Float) (Variables|Default|GetZoomSize))))

(event Input|EnhancedActionEvents|EnhancedInputActionIA_MoveDown
  (params (ActionValue :type Float%20%28double-precision%29) (ElapsedSeconds :type Float%20%28double-precision%29) (TriggeredSeconds :type Float%20%28double-precision%29) (InputAction :type Input%20Action%20Object%20Reference :default "/Game/InputActions/IA_MoveDown.IA_MoveDown"))
  (CallFunction|BPMove (* ActionValue -1.0) 0.0 (/ (Variables|Default|GetZoomSize) 3e+02)))

(event Input|EnhancedActionEvents|EnhancedInputActionIA_MoveUp
  (params (ActionValue :type Float%20%28double-precision%29) (ElapsedSeconds :type Float%20%28double-precision%29) (TriggeredSeconds :type Float%20%28double-precision%29) (InputAction :type Input%20Action%20Object%20Reference :default "/Game/InputActions/IA_MoveUp.IA_MoveUp"))
  (CallFunction|BPMove ActionValue 0.0 (/ (Variables|Default|GetZoomSize) 3e+02)))

(event Input|EnhancedActionEvents|EnhancedInputActionIA_PlaceCircuitComponent
  (params (ActionValue :type Boolean) (ElapsedSeconds :type Float%20%28double-precision%29) (TriggeredSeconds :type Float%20%28double-precision%29) (InputAction :type Input%20Action%20Object%20Reference :default "/Game/InputActions/IA_PlaceCircuitComponent.IA_PlaceCircuitComponent"))
  (:Started
    (CallFunction|BPPlaceComponent)))

(event Input|EnhancedActionEvents|EnhancedInputActionIA_MoveLeft
  (params (ActionValue :type Float%20%28double-precision%29) (ElapsedSeconds :type Float%20%28double-precision%29) (TriggeredSeconds :type Float%20%28double-precision%29) (InputAction :type Input%20Action%20Object%20Reference :default "/Game/InputActions/IA_MoveLeft.IA_MoveLeft"))
  (CallFunction|BPMove 0.0 (* ActionValue -1.0) (/ (Variables|Default|GetZoomSize) 3e+02)))

(event Input|EnhancedActionEvents|EnhancedInputActionIA_MoveRight
  (params (ActionValue :type Float%20%28double-precision%29) (ElapsedSeconds :type Float%20%28double-precision%29) (TriggeredSeconds :type Float%20%28double-precision%29) (InputAction :type Input%20Action%20Object%20Reference :default "/Game/InputActions/IA_MoveRight.IA_MoveRight"))
  (CallFunction|BPMove 0.0 ActionValue (/ (Variables|Default|GetZoomSize) 3e+02)))

(event EventTick
  (params (DeltaSeconds :type Float%20%28single-precision%29)))

(event EventBeginPlay
  (Utilities|FlowControl|Sequence
    (:then_0
      (Input|AddMappingContext (PlayerController|LocalPlayerSubsystems|GetEnhancedInputLocalPlayerSubsystem self) "/Game/InputMappingContext/IMC_DesignLuminaCircuit.IMC_DesignLuminaCircuit" 0 "(bIgnoreAllPressedKeysUntilRelease=True,bForceImmediately=False,bNotifyUserSettings=False)"))
    (:then_1
      (bind _asc_design_lumina_circuit_character (Utilities|Casting|CastToC_DesignLuminaCircuitCharacter (Pawn|GetControlledPawn)))
      (Default|SetCameraScreenSize _asc_design_lumina_circuit_character (Variables|Default|GetZoomSize)))
    (:then_2
      (Variables|Default|SetbShowMouseCursor true))))

(fn ConstructionScript)

(fn BPMove
  (params (UpPositiveValue :type Float%20%28double-precision%29) (RightPositiveValue :type Float%20%28double-precision%29) (Speed :type Float%20%28double-precision%29))
  (Class|CPPPCDesignLuminaCircuit|Move UpPositiveValue RightPositiveValue Speed))

(fn BPZoom
  (params (Value :type Float%20%28double-precision%29))
  (LocalVariables|SetWidth Value)
  (bind _asc_design_lumina_circuit_character (Utilities|Casting|CastToC_DesignLuminaCircuitCharacter (Pawn|GetControlledPawn)))
  (Default|SetCameraScreenSize _asc_design_lumina_circuit_character (LocalVariables|GetWidth)))

(fn BPPlaceComponent
  (Class|CPPPCDesignLuminaCircuit|PlaceComponent 5e+03)
  (Development|PrintString "Hello"))