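; Player controller for the survival character, handling movement, jump, item use and the energy bar HUD.
; BeginPlay caches BP_MainCharacter, retrying each tick until the cast succeeds, adds the input mapping context and creates W_EnergyBar.
; Move inputs overwrite horizontal velocity along cached flattened forward/right vectors, which rotation input recomputes after yawing the character.
; Jump applies a grounded-only impulse, and Use messages the closest detected actor through BPI_CanUse.
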(event Input|EnhancedActionEvents|EnhancedInputActionIA_MoveUp
  (params (ActionValue :type Float%20%28double-precision%29) (ElapsedSeconds :type Float%20%28double-precision%29) (TriggeredSeconds :type Float%20%28double-precision%29) (InputAction :type Input%20Action%20Object%20Reference :default "/Game/InputActions/IA_MoveUp.IA_MoveUp"))
  (bind _as_bp_main_character (Variables|Default|GetAs%20BP%20Main%20Character)
    (:then
      (Variables|/Script/Engine.MovementComponent|SetVelocity (Variables|/Script/Engine.Character|GetCharacterMovement _as_bp_main_character) (+ (Math|Vector|MakeVector 0.0 0.0 (.z (Pawn|Components|CharacterMovement|GetLastUpdateVelocity (Variables|/Script/Engine.Character|GetCharacterMovement _as_bp_main_character)))) (* (Variables|Default|GetForwardVector) (* ActionValue (Variables|Default|GetSpeed))))))
    (:else)))

(event Input|EnhancedActionEvents|EnhancedInputActionIA_MoveDown
  (params (ActionValue :type Float%20%28double-precision%29) (ElapsedSeconds :type Float%20%28double-precision%29) (TriggeredSeconds :type Float%20%28double-precision%29) (InputAction :type Input%20Action%20Object%20Reference :default "/Game/InputActions/IA_MoveDown.IA_MoveDown"))
  (bind _as_bp_main_character (Variables|Default|GetAs%20BP%20Main%20Character)
    (:then
      (Variables|/Script/Engine.MovementComponent|SetVelocity (Variables|/Script/Engine.Character|GetCharacterMovement _as_bp_main_character) (+ (Math|Vector|MakeVector 0.0 0.0 (.z (Pawn|Components|CharacterMovement|GetLastUpdateVelocity (Variables|/Script/Engine.Character|GetCharacterMovement _as_bp_main_character)))) (* (Variables|Default|GetForwardVector) (* (* ActionValue (Variables|Default|GetSpeed)) -1.0)))))
    (:else)))

(event Input|EnhancedActionEvents|EnhancedInputActionIA_Use
  (params (ActionValue :type Boolean) (ElapsedSeconds :type Float%20%28double-precision%29) (TriggeredSeconds :type Float%20%28double-precision%29) (InputAction :type Input%20Action%20Object%20Reference :default "/Game/InputActions/IA_Use.IA_Use"))
  (:Started
    (Utilities|FlowControl|Sequence
      (:then_0
        (bind _as_bp_main_character (Variables|Default|GetAs%20BP%20Main%20Character)
          (:then
            (bind _closestdetectedactor (Default|GetClosestDetectedActor _as_bp_main_character))
            (if (Utilities|DoesObjectImplementInterface _closestdetectedactor "/Game/Interfaces/BPI_CanUse.BPI_CanUse_C")
              (Class|BPICanUse|Use(Message) _closestdetectedactor self)
              (else
                (CallFunction|LogInfo "PC_StartMain" "This Item Cannot Be Used"))))
          (:else))))))

(event Input|EnhancedActionEvents|EnhancedInputActionIA_MoveRight
  (params (ActionValue :type Float%20%28double-precision%29) (ElapsedSeconds :type Float%20%28double-precision%29) (TriggeredSeconds :type Float%20%28double-precision%29) (InputAction :type Input%20Action%20Object%20Reference :default "/Game/InputActions/IA_MoveRight.IA_MoveRight"))
  (bind _as_bp_main_character (Variables|Default|GetAs%20BP%20Main%20Character)
    (:then
      (Variables|/Script/Engine.MovementComponent|SetVelocity (Variables|/Script/Engine.Character|GetCharacterMovement _as_bp_main_character) (+ (Math|Vector|MakeVector 0.0 0.0 (.z (Pawn|Components|CharacterMovement|GetLastUpdateVelocity (Variables|/Script/Engine.Character|GetCharacterMovement _as_bp_main_character)))) (* (Variables|Default|GetRightVector) (* ActionValue (Variables|Default|GetSpeed))))))
    (:else)))

(event Input|EnhancedActionEvents|EnhancedInputActionIA_MoveLeft
  (params (ActionValue :type Float%20%28double-precision%29) (ElapsedSeconds :type Float%20%28double-precision%29) (TriggeredSeconds :type Float%20%28double-precision%29) (InputAction :type Input%20Action%20Object%20Reference :default "/Game/InputActions/IA_MoveLeft.IA_MoveLeft"))
  (bind _as_bp_main_character (Variables|Default|GetAs%20BP%20Main%20Character)
    (:then
      (Variables|/Script/Engine.MovementComponent|SetVelocity (Variables|/Script/Engine.Character|GetCharacterMovement _as_bp_main_character) (+ (Math|Vector|MakeVector 0.0 0.0 (.z (Pawn|Components|CharacterMovement|GetLastUpdateVelocity (Variables|/Script/Engine.Character|GetCharacterMovement _as_bp_main_character)))) (* (Variables|Default|GetRightVector) (* (* ActionValue (Variables|Default|GetSpeed)) -1.0)))))
    (:else)))

(event Input|EnhancedActionEvents|EnhancedInputActionIA_RotateCamera
  (params (ActionValue :type Float%20%28double-precision%29) (ElapsedSeconds :type Float%20%28double-precision%29) (TriggeredSeconds :type Float%20%28double-precision%29) (InputAction :type Input%20Action%20Object%20Reference :default "/Game/InputActions/IA_RotateCamera.IA_RotateCamera"))
  (bind _as_bp_main_character (Variables|Default|GetAs%20BP%20Main%20Character)
    (:then
      (Transformation|AddActorLocalRotation _as_bp_main_character (Math|Rotator|MakeRotator 0.0 0.0 (* ActionValue 1.0)) false false)
      (CallFunction|SetForwardVector _as_bp_main_character)
      (CallFunction|SetRightVector))
    (:else)))

(event Input|EnhancedActionEvents|EnhancedInputActionIA_Jump
  (params (ActionValue :type Boolean) (ElapsedSeconds :type Float%20%28double-precision%29) (TriggeredSeconds :type Float%20%28double-precision%29) (InputAction :type Input%20Action%20Object%20Reference :default "/Game/InputActions/IA_Jump.IA_Jump"))
  (:Started
    (bind _as_bp_main_character (Variables|Default|GetAs%20BP%20Main%20Character)
      (:then
        (if (AI|Components|NavMovement|IsMovingonGround (Variables|/Script/Engine.Character|GetCharacterMovement _as_bp_main_character))
          (Physics|AddImpulse (Variables|/Script/Engine.Character|GetCharacterMovement _as_bp_main_character) "0.000000,0.000000,80000.000000" false)))
      (:else))))

(event EventBeginPlay
  (bind _self self)
  (bind _returnvalue (PlayerController|LocalPlayerSubsystems|GetEnhancedInputLocalPlayerSubsystem _self))
  (Utilities|FlowControl|Sequence
    (:then_0
      ;[1 1 1] Get Main Character
      (bind _asbp_main_character (Utilities|Casting|CastToBP_MainCharacter (Pawn|GetControlledPawn self) :!label _label)
        (:then
          (bind _output_get (Variables|Default|SetAs%20BP%20Main%20Character _asbp_main_character))
          (CallFunction|LogInfo _output_get "BP Main Character Set!"))
        (:CastFailed
          (Utilities|FlowControl|DelayUntilNextTick)
          (goto _label))))
    (:then_1
      ;[1 1 1] Add Mapping Context
      (Utilities|IsValid _returnvalue
        (:Is%20Valid
          (Input|AddMappingContext _returnvalue "/Game/InputMappingContext/IMC_MainSurvival.IMC_MainSurvival" 0 "(bIgnoreAllPressedKeysUntilRelease=True,bForceImmediately=False,bNotifyUserSettings=False)")
          (CallFunction|LogInfo self "Added Mapping Context"))))
    (:then_2
      ;[1 1 1] Set Up Vector
      (bind _as_bp_main_character (Variables|Default|GetAs%20BP%20Main%20Character)
        (:then
          (CallFunction|SetForwardVector _as_bp_main_character)
          (CallFunction|SetRightVector))
        (:else)))
    (:then_3
      (bind _returnvalue_2 (UserInterface|CreateWidget "/Game/Widgets/W_EnergyBar.W_EnergyBar_C"))
      (bind _output_get_2 (Variables|Default|SetEnergyBar _returnvalue_2))
      (UserInterface|Viewport|AddtoViewport _output_get_2 0))))

(fn ConstructionScript)

(fn SetForwardVector
  (params (MainCharacter :type Actor%20Object%20Reference))
  (bind _returnvalue (Transformation|GetActorRotation MainCharacter))
  (bind _returnvalue_2 (Math|Vector|GetForwardVector _returnvalue))
  (Variables|Default|SetForwardVector (Math|Vector|Normalize (Math|Vector|MakeVector (.x _returnvalue_2) (.y _returnvalue_2) 0.0))))

(fn SetRightVector
  (Variables|Default|SetRightVector (Math|Vector|RotateVectorAroundAxis (Variables|Default|GetForwardVector) 9e+01 "0.000000,0.000000,1.000000")))

(fn GetBPMainCharacter
  (return (Variables|Default|GetAs%20BP%20Main%20Character)))

(fn GetSleepBPBed
  (return (Variables|Default|GetSleepBPBed)))

(fn GetPlayerCameraManager
  (bind _playercameramanager (Variables|Default|GetPlayerCameraManager)
    (:then
      (return _playercameramanager))
    (:else)))

(fn GetPlayerState
  (bind _playerstate (Variables|GetPlayerState)
    (:then
      (return _playerstate))
    (:else
      (CallFunction|LogInfo "PC_StartMain" "PlayerState Not Found"))))

(fn GetEnergyBar
  (return (Variables|Default|GetEnergyBar)))